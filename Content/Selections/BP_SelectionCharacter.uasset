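; BP_SelectionCharacter is a character selection Blueprint that cycles its mesh through a list of skeletal meshes.
; Pressing the 5 key calls RPCPlaySelection, which runs ChangeCharacter to advance the index, wrapping to the first entry at the end.
; The chosen mesh is applied to the Mesh component and stored in the GI_Selection game instance as SkeletalMeshSelected.
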(event `RPC Play Selection`
  (`self.Change Character`))

(event `Key|Five`
  (params (Key :type "Key Structure"))
  (:`Pressed`
    (`self.RPC Play Selection`)))

(event `Change Character`
  (bind _output (`|GetArrayItem` (`self.characters`) (`self.currentCharacterIndex`)))
  (if (< (`self.currentCharacterIndex`) (- (`KismetArrayLibrary.Array_Length` (`self.characters`)) 1))
    (`/Engine/EditorBlueprintResources/StandardMacros.IncrementInt` (`self.currentCharacterIndex`)
      (:`  `
        _))
    (else
      (set `self.currentCharacterIndex` 0)))
  (`SkeletalMeshComponent.SetSkeletalMeshAsset` (`self.Mesh`) _output)
  (bind _asgi_selection (cast `/Game/Selections/GI_Selection` (`GameplayStatics.GetGameInstance`)))
  (set `/Game/Selections/GI_Selection.skeletalMeshSelected` _output _asgi_selection))

(fn `UserConstructionScript`)